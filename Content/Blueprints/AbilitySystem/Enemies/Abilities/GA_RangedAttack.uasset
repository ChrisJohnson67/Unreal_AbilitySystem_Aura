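; GA_RangedAttack is an enemy gameplay ability that fires a projectile at the avatar's combat target.
; On activation it captures the target's location, turns the avatar toward it via interface messages, and plays a random tagged attack montage.
; The montage's matching gameplay event triggers SpawnProjectile toward that captured location, and the ability ends after a short delay.
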(event Ability|EventActivateAbility
  (bind _returnvalue (Class|EnemyInterface|GetCombatTarget(Message) (Ability|GetAvatarActorfromActorInfo)))
  (Variables|Default|SetProjectileTargetLoc (Transformation|GetActorLocation _returnvalue))
  (Class|CombatInterface|UpdateFacingTarget(Message) (Ability|GetAvatarActorfromActorInfo) (Variables|Default|GetProjectileTargetLoc))
  (bind _returnvalue_2 (Class|CombatInterface|GetAttackMontages(Message) (Ability|GetAvatarActorfromActorInfo)))
  (Variables|Default|SetTaggedMontage (Class|AuraDamageGameplayAbility|GetRandomTaggedMontagefromArray _returnvalue_2))
  (|PlayMontageandWaitProxy "None" (.Montage (Utilities|Struct|BreakTaggedMontage (Variables|Default|GetTaggedMontage))) 1.0 "None" false 1.0 0.0 false
    (:then
      (Ability|Tasks|WaitGameplayEvent (.MontageTag (Utilities|Struct|BreakTaggedMontage (Variables|Default|GetTaggedMontage))) 0
        (:EventReceived
          (Class|CombatInterface|GetCombatSocketLocation(Message) (Ability|GetAvatarActorfromActorInfo) (.MontageTag (Utilities|Struct|BreakTaggedMontage (Variables|Default|GetTaggedMontage))))
          (Class|AuraProjectileSpell|SpawnProjectile (Variables|Default|GetProjectileTargetLoc))
          (Utilities|FlowControl|Delay 0.2)
          (Ability|EndAbility))))))

(event Ability|EventOnEndAbility
  (params (bWasCancelled :type Boolean)))